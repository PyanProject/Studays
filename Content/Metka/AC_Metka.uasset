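; AC_Metka is a marker actor with a widget display that disappears when the player's ThirdPersonCharacter touches it.
; On BeginPlay it sets its actor tag to MyTag and uses that as the row key into the Metka_tab data table.
; The row supplies the texture and name for its WG_Metka widget, which also receives the tag.
; Overlap with its Sphere component by that character destroys the actor.
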(event OnComponentBeginOverlap(Sphere)
  (params (OverlappedComponent :type Primitive%20Component%20Object%20Reference) (OtherActor :type Actor%20Object%20Reference) (OtherComp :type Primitive%20Component%20Object%20Reference) (OtherBodyIndex :type Integer) (bFromSweep :type Boolean) (SweepResult :type Hit%20Result%20Structure%20%28by%20ref%29))
  (Utilities|Casting|CastToThirdPersonCharacter OtherActor)
  (Actor|DestroyActor))

(event EventBeginPlay
  (bind _mytag (Variables|Default|GetMyTag))
  (bind _aswg_metka (Utilities|Casting|CastToWG_Metka (UserInterface|GetWidget (Variables|Default|GetWidget))))
  (Variables|Default|SetTags (Utilities|Array|MakeArray _mytag))
  (bind _returnvalue (Utilities|GetDataTableRow "/Game/Metka/Metka_tab.Metka_tab" _mytag)
    (:then
      (Appearance|SetBrushfromTexture (Variables|/Game/Metka/WG_Metka.WG_Metka_C|GetImage_0 _aswg_metka) (.Texture (Utilities|Struct|BreakMetka_Str _returnvalue)) false)
      (Variables|/Game/Metka/WG_Metka.WG_Metka_C|SetTag _aswg_metka _mytag)
      (Rendering|Components|TextRender|SetText (Variables|/Game/Metka/WG_Metka.WG_Metka_C|GetTextBlock_1 _aswg_metka) (Utilities|Text|ToText(Name) (.Name (Utilities|Struct|BreakMetka_Str _returnvalue)))))))

(fn ConstructionScript)