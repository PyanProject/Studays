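; Timed-mission actor that starts a minutes:seconds countdown when the ThirdPersonCharacter enters its Box trigger.
; The overlap creates the WG_Timer widget and enables Tick, which decrements one second per call, so pacing depends on tick rate.
; At zero, Finish shows the result overlay with cursor and UI-only input, then stops Tick.
; MisComplete, set outside this graph, selects success text and time reset, or a brief player input lock.
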(event OnComponentBeginOverlap(Box)
  (params (OverlappedComponent :type Primitive%20Component%20Object%20Reference) (OtherActor :type Actor%20Object%20Reference) (OtherComp :type Primitive%20Component%20Object%20Reference) (OtherBodyIndex :type Integer) (bFromSweep :type Boolean) (SweepResult :type Hit%20Result%20Structure%20%28by%20ref%29))
  (Utilities|Casting|CastToThirdPersonCharacter OtherActor)
  (Utilities|FlowControl|DoOnce false :!label _label
    (:Completed
      (bind _returnvalue (UserInterface|CreateWidget "/Game/Метка(ТАЙМЕР)/Mission/WG_Timer.WG_Timer_C"))
      (bind _output_get (Variables|Default|SetWG_Timer _returnvalue))
      (UserInterface|Viewport|AddtoViewport _output_get 0)
      (Variables|Default|SetGoMis true)
      (Development|SetHiddeninGame (Variables|Default|GetBox) false false)
      (Actor|Tick|SetActorTickEnabled true)
      (Utilities|FlowControl|Delay 0.2)
      (goto _label Reset))))

(event Custom|Finish
  (bind _returnvalue (Game|GetPlayerController 0))
  (bind _wg_timer (Variables|Default|GetWG_Timer))
  (bind _nogood_overlay (Variables|/Game/Метка(ТАЙМЕР)/Mission/WG_Timer.WG_Timer_C|GetNoGOOD_overlay _wg_timer))
  (if (Variables|Default|GetMisComplete)
    (Widget|SetVisibility _nogood_overlay "Visible")
    (Rendering|Components|TextRender|SetText (Variables|/Game/Метка(ТАЙМЕР)/Mission/WG_Timer.WG_Timer_C|GetTextButton _wg_timer) "Закрыть")
    (Rendering|Components|TextRender|SetText (Variables|/Game/Метка(ТАЙМЕР)/Mission/WG_Timer.WG_Timer_C|GetTextMission _wg_timer) "Вы отлично выполнили миссию")
    (Variables|/Script/Engine.PlayerController|SetbShowMouseCursor _returnvalue true)
    (Input|SetInputModeUIOnly _returnvalue _wg_timer "DoNotLock")
    (Rendering|SetVisibility (Variables|Default|GetBox) true false)
    (Variables|Default|SetSec (Variables|Default|GetSec_0))
    (Variables|Default|SetMin (Variables|Default|GetMin_0))
    (else
      (Widget|SetVisibility _nogood_overlay "Visible")
      (Variables|/Script/Engine.PlayerController|SetbShowMouseCursor _returnvalue true)
      (Input|SetInputModeUIOnly _returnvalue _wg_timer "DoNotLock")
      (Input|DisableInput (Game|GetPlayerCharacter 0) (Game|GetPlayerController 0))
      (Utilities|FlowControl|Delay 1.5)))
  (Widget|SetVisibility (Variables|/Game/Метка(ТАЙМЕР)/Mission/WG_Timer.WG_Timer_C|GetOverlay_0 (Variables|Default|GetWG_Timer)) "Visible")
  (Actor|Tick|SetActorTickEnabled false)
  (Input|EnableInput (Game|GetPlayerCharacter 0) (Game|GetPlayerController 0)))

(event EventBeginPlay
  (Actor|Tick|SetActorTickEnabled false)
  (bind _output_get (Variables|Default|SetSec (Math|Integer|Clamp(Integer) (Variables|Default|GetSec) 0 59)))
  (Variables|Default|SetSec_0 _output_get)
  (bind _output_get_2 (Variables|Default|SetMin (Math|Integer|Clamp(Integer) (Variables|Default|GetMin) 0 59)))
  (Variables|Default|SetMin_0 _output_get_2))

(event EventTick
  (params (DeltaSeconds :type Float%20%28single-precision%29))
  (if (Variables|Default|GetGoMis)
    (if (== (Variables|Default|GetSec) 0)
      (if (== (Variables|Default|GetMin) 0)
        (Utilities|FlowControl|Delay 0.2)
        (CallFunction|Finish)
        (else
          (Variables|Default|SetSec 59)
          (bind _result (Math|Integer|DecrementInt (Variables|Default|GetMin))
            (:%20%20
              (Variables|Default|SetMin _result)))))
      (else
        (bind _result_2 (Math|Integer|DecrementInt (Variables|Default|GetSec))
          (:%20%20
            (Variables|Default|SetSec _result_2)))))))

(fn ConstructionScript)